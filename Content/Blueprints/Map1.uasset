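; Map1 is an actor that treats its mesh as a sphere and provides surface queries for points around it.
; The construction script caches the mesh bounds' sphere radius in Unreal units and in meters.
; GetSurfaceLocationAndNormal returns the center-to-point direction as the normal, and that direction scaled by radius plus the negated actor location as the surface location.
; The event graph is unused.
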(fn `Get Surface Location and Normal`
  (params (Location :type "Vector Structure"))
  (returns (`Surface Location` :type "Vector Structure") (`Surface Normal` :type "Vector Structure"))
  (bind _returnvalue (* (`KismetMathLibrary.Normal` (- (`self.K2_GetActorLocation`) Location)) -1.0))
  ;[1 1 1] must be in the main class
  (return (+ (* _returnvalue (`self.Radius(units)`)) (* (`self.K2_GetActorLocation`) -1.0)) _returnvalue))

(fn `UserConstructionScript`
  (bind _output_get (set `self.Radius(units)` (`.SphereRadius` (`KismetSystemLibrary.GetComponentBounds` (`self.MeshComponent`)))))
  (set `self.Radius(m)` (/ _output_get 100.0)))