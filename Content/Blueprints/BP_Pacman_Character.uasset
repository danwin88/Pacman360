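; VR player character for a Pac-Man game that drives a separate Pacman actor over a spherical map, starting paused with a floor tracking origin.
; D-pad input sets the offset applied each unpaused tick, then Pacman is re-projected near the map radius and oriented to its surface.
; Tick also refreshes the score text.
; Keys, mouse, controller and taps click widgets; swipe and axis-movement handlers are empty stubs.
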(event `self.ReceiveBeginPlay`
  ;[0 0 0] Begin Play
  (`HeadMountedDisplayFunctionLibrary.SetTrackingOrigin` "Floor")
  (bind _outactors (`GameplayStatics.GetAllActorsOfClass` "/Game/Blueprints/Pacman.Pacman_C"))
  (set `self.Pacman` (`|GetArrayItem` _outactors))
  (bind _outactors_2 (`GameplayStatics.GetAllActorsOfClass` "/Game/Blueprints/Map1.Map1_C"))
  (set `self.Map` (`|GetArrayItem` _outactors_2))
  (`ActorComponent.SetTickableWhenPaused` (`self.FirstPersonCameraComponent`) true)
  (`self.SetTickableWhenPaused` self true)
  (bind _returnvalue (`GameplayStatics.SetGamePaused` true))
  (set `self.Game Paused?` _returnvalue))

(event `Key|AnyKey`
  (params (Key :type "Key Structure"))
  (bind _widgetinteraction (`self.WidgetInteraction`))
  (:`Pressed`
    (`WidgetInteractionComponent.PressPointerKey` _widgetinteraction "LeftMouseButton" :!label _label))
  (:`Released`
    (`WidgetInteractionComponent.ReleasePointerKey` _widgetinteraction "LeftMouseButton" :!label _label_2)))

(event `self.ReceiveTick`
  (params (DeltaSeconds :type "Float (single-precision)"))
  (bind _map (`self.Map`))
  (bind _pacman (`self.Pacman`))
  (bind _returnvalue (`KismetMathLibrary.Normal` (- (`self.K2_GetActorLocation` _map) (`self.K2_GetActorLocation` _pacman))))
  ;[1 1 1] Tick
  (bind _returnvalue_2 (`self.GetScore`))
  (`TextRenderComponent.K2_SetText` (`self.ScreenScore`) (`KismetTextLibrary.Conv_IntToText` _returnvalue_2))
  (if (not (`self.Game Paused?`))
    (`self.K2_AddActorLocalOffset` _pacman (* (`KismetMathLibrary.ClampVectorSize` (`KismetMathLibrary.MakeVector` (`self.x`) (`self.y`)) 0.0 1.0) (* DeltaSeconds (`self.velocity`))) false false)
    (`self.K2_SetActorLocationAndRotation` _pacman (+ (* (* _returnvalue -1.0) (- (`/Game/Blueprints/Map1.Radius(units)` _map) 40.0)) (* (`self.K2_GetActorLocation` _map) -1.0)) (`KismetMathLibrary.MakeRotFromZY` _returnvalue (`self.GetActorRightVector`)) false false)))

(event `Key|MotionController_Right_FaceButton1` :paused true
  (params (Key :type "Key Structure"))
  (:`Pressed`
    (goto _label))
  (:`Released`
    (goto _label_2)))

(event `InputTouch` :paused true
  (params (Location :type "Vector Structure") (FingerIndex :type "ETouchIndex Enum"))
  (bind _widgetinteraction (`self.WidgetInteraction`))
  (bind _returnvalue (- (`self.Touch Start`) (`self.Touch End`)))
  (bind (_locationx _locationy) (`PlayerController.GetInputTouchState` (`GameplayStatics.GetPlayerController` 0) "Touch1"))
  (bind _returnvalue_2 (`KismetMathLibrary.MakeVector2D` _locationx _locationy))
  (bind (_x _y) (`KismetMathLibrary.BreakVector2D` _returnvalue))
  (:`Pressed`
    (set `self.Touch Start` _returnvalue_2))
  (:`Released`
    (set `self.Touch End` _returnvalue_2)
    ;[1 1 1] touch pad
    (if (> (`KismetMathLibrary.VSize2D` _returnvalue) 20.0)
      (if (> (`KismetMathLibrary.Abs` _x) (`KismetMathLibrary.Abs` _y))
        ;[1 1 1] right
        (if true
          _)
        (else
          ;[1 1 1] VR Input Menu
          ;;[1 1 1] up
          (if true
            _)))
      (else
        (`WidgetInteractionComponent.PressPointerKey` _widgetinteraction "LeftMouseButton")
        (`WidgetInteractionComponent.ReleasePointerKey` _widgetinteraction "LeftMouseButton")))))

(event `Key|Gamepad_DPad_Up`
  (params (Key :type "Key Structure"))
  (:`Pressed`
    (set `self.x` 1.0))
  (:`Released`
    (set `self.x` 0.0)))

(event `Key|Gamepad_DPad_Down`
  (params (Key :type "Key Structure"))
  (:`Pressed`
    (set `self.x` -1.0))
  (:`Released`
    (set `self.x` 0.0)))

(event `Key|Gamepad_DPad_Right`
  (params (Key :type "Key Structure"))
  (:`Pressed`
    (set `self.y` 1.0))
  (:`Released`
    (set `self.y` 0.0)))

(event `Key|Gamepad_DPad_Left`
  (params (Key :type "Key Structure"))
  (:`Pressed`
    (set `self.y` -1.0))
  (:`Released`
    (set `self.y` 0.0)))

(event `InputAxis|MoveForward`
  (params (AxisValue :type "Float (single-precision)"))
  ;[1 1 1] Movement fix
  (if (> AxisValue (stale `InputAxis|MoveRight` AxisValue)) :!label _label_3
    _))

(event `InputAxis|MoveRight`
  (params (AxisValue :type "Float (single-precision)"))
  ;[1 1 1] Movement fix
  (goto _label_3))

(event `Key|LeftMouseButton` :paused true
  (params (Key :type "Key Structure"))
  (bind _widgetinteraction (`self.WidgetInteraction`))
  ;[1 1 1] VR Input Menu
  (:`Pressed`
    (`WidgetInteractionComponent.PressPointerKey` _widgetinteraction "LeftMouseButton"))
  (:`Released`
    (`WidgetInteractionComponent.ReleasePointerKey` _widgetinteraction "LeftMouseButton")))

(fn `UserConstructionScript`)