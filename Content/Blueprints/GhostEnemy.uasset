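; Ghost enemy for a Pac-Man game on a spherical map, scoring when eaten while vulnerable, otherwise saving any best score and restarting the level.
; Tick steers straight at a close Pacman, else toward a PathPoint, then snaps and orients the ghost to the sphere.
; GetClosetPoint line-traces nearby shuffled points, favouring those nearer Pacman, or farther when CanTakeDamage.
; Spline, AIMoveTo and other movement experiments remain unconnected.
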(event `self.ReceiveActorBeginOverlap`
  (params (OtherActor :type "Actor Object Reference"))
  ;[1 1 1] Actor overlap
  (bind _aspacman (cast `/Game/Blueprints/Pacman` OtherActor))
  (if (and (`self.bCanTakeDamage`) (`PrimitiveComponent.IsOverlappingActor` (`self.Capsule`) _aspacman))
    (bind _asbp_pacman_character (cast `/Game/Blueprints/BP_Pacman_Character` (`GameplayStatics.GetPlayerCharacter` 0)))
    (bind _returnvalue (`self.GetScore`))
    (`GearVRCharacter.UpdateScore` _asbp_pacman_character _returnvalue)
    (`self.K2_DestroyActor`)
    (else
      (bind _returnvalue_2 (`GameplayStatics.LoadGameFromSlot` "MySave"))
      (bind _asgear_vrsave_game (cast `/Game/Blueprints/GearVRSaveGame` _returnvalue_2))
      (bind _asbp_pacman_character_2 (cast `/Game/Blueprints/BP_Pacman_Character` (`GameplayStatics.GetPlayerCharacter` 0))
        (:`then`
          (bind _score (`GearVRCharacter.Score` _asbp_pacman_character_2))
          (if (> _score (`/Game/Blueprints/GearVRSaveGame.Best Score` _asgear_vrsave_game))
            (bind _returnvalue_3 (`GameplayStatics.CreateSaveGameObject` "/Game/Blueprints/GearVRSaveGame.GearVRSaveGame_C"))
            (set `/Game/Blueprints/GearVRSaveGame.Best Score` _score _returnvalue_3)
            (`GameplayStatics.SaveGameToSlot` _returnvalue_3 "MySave")))
        (:`CastFailed`
          _))
      (bind _asbp_gear_vrgame_game_mode_base (cast `/Game/Blueprints/BP_GearVRGameGameModeBase` (`GameplayStatics.GetGameMode`)))
      (`GameModeBase.ResetLevel` _asbp_gear_vrgame_game_mode_base)
      (`GameMode.RestartGame` _asbp_gear_vrgame_game_mode_base))))

(event `self.ReceiveBeginPlay`
  ;[1 1 1] Begin Play
  (bind _outactors (`GameplayStatics.GetAllActorsOfClass` "/Game/Blueprints/Pacman.Pacman_C"))
  (set `self.Pacman` (`|GetArrayItem` _outactors))
  (bind _outactors_2 (`GameplayStatics.GetAllActorsOfClass` "/Game/Blueprints/Map1.Map1_C"))
  (set `self.Map` (`|GetArrayItem` _outactors_2))
  (bind _outactors_3 (`GameplayStatics.GetAllActorsOfClass` "/Game/Blueprints/PathPoint.PathPoint_C"))
  (set `self.PathPoints` _outactors_3))

(event `self.ReceiveTick`
  (params (DeltaSeconds :type "Float (single-precision)"))
  (bind _map (`self.Map`))
  (bind _returnvalue (- (`self.K2_GetActorLocation` (`self.Pacman`)) (`self.K2_GetActorLocation`)))
  (bind _returnvalue_2 (`KismetMathLibrary.Normal` (- (`self.K2_GetActorLocation` _map) (`self.K2_GetActorLocation`))))
  ;[1 0.125 0.125] AI Movement
  (if (<= (`KismetMathLibrary.VSize` _returnvalue) 150.0)
    (`self.K2_AddActorLocalOffset` (* (* (`KismetMathLibrary.Normal` _returnvalue) (`self.Velocity`)) DeltaSeconds))
    (else
      (`self.K2_AddActorLocalOffset` (* (* (`KismetMathLibrary.Normal` (- (`self.K2_GetActorLocation` (`self.Get Closet Point`)) (`self.K2_GetActorLocation`))) (`self.Velocity`)) DeltaSeconds))))
  (`self.K2_SetActorLocationAndRotation` (+ (* (* _returnvalue_2 -1.0) (- (`/Game/Blueprints/Map1.Radius(units)` _map) 80.0)) (* (`self.K2_GetActorLocation` _map) -1.0)) (`KismetMathLibrary.MakeRotFromZY` _returnvalue_2 (`self.GetActorRightVector`))))

(fn `Get Closet Point`
  (returns (`Closest Point` :type "/Game/Blueprints/PathPoint Object Reference"))
  (locals (`Closet point` :type "/Game/Blueprints/PathPoint Object Reference") (NearPoints :type "Array of /Game/Blueprints/PathPoint Object Reference") (Open :type "Array of /Game/Blueprints/PathPoint Object Reference") (Closed :type "Array of /Game/Blueprints/PathPoint Object Reference") (CurrentPoint :type "/Game/Blueprints/PathPoint Object Reference") (fScore :type "Float (double-precision)") (tentative_gScore :type "Float (double-precision)"))
  (bind _nearpoints (`local.NearPoints`))
  (bind _closet_point (`local.Closet point`))
  (bind _output (`|GetArrayItem` _nearpoints))
  (`KismetArrayLibrary.Array_Shuffle` (`self.PathPoints`))
  (set `self.Min` 0.0)
  (`KismetArrayLibrary.Array_Clear` (`local.NearPoints`))
  (for _index (range (`KismetArrayLibrary.Array_Length` (`self.PathPoints`)))
    (bind _output_2 (`|GetArrayItem` (`self.PathPoints`) _index))
    (if (< (`KismetMathLibrary.VSize` (- (`self.K2_GetActorLocation` _output_2) (`self.K2_GetActorLocation`))) 300.0)
      (`KismetArrayLibrary.Array_Add` (`local.NearPoints`) _output_2)))
  (`KismetArrayLibrary.Array_Shuffle` _nearpoints)
  (set `local.Closet point` _output)
  (set `self.Min` (`KismetMathLibrary.VSize` (- (`self.K2_GetActorLocation` (`self.Pacman`)) (`self.K2_GetActorLocation` _output))))
  (for _index_2 (range (`KismetArrayLibrary.Array_Length` (`local.NearPoints`)))
    (if (`self.bCanTakeDamage`)
      (bind _output_3 (`|GetArrayItem` (`local.NearPoints`) _index_2))
      (if (< (`self.Min`) (`KismetMathLibrary.VSize` (- (`self.K2_GetActorLocation` (`self.Pacman`)) (`self.K2_GetActorLocation` _output_3))))
        (bind _outactors (`GameplayStatics.GetAllActorsOfClass` "/Script/GearVRGame.GoalPickup" :!label _label))
        (bind _outhit (`KismetSystemLibrary.LineTraceSingleForObjects` (`self.K2_GetActorLocation`) (`self.K2_GetActorLocation` _output_3) (`|MakeArray` "ObjectTypeQuery1" "ObjectTypeQuery2" :!type "EObjectTypeQuery Enum") true _outactors "None" true (struct :`R` 0.141643 :`B` 1.0 :`A` 1.0) (struct :`R` 0.95157 :`G` 0.943905 :`B` 1.0 :`A` 1.0)))
        (bind (_bblockinghit _binitialoverlap _time _location _impactpoint _normal _impactnormal _physmat _hitactor) (`GameplayStatics.BreakHitResult` _outhit))
        ;[1 1 1] Can See The point
        (cast `/Game/Blueprints/PathPoint` _hitactor
          (:`then`
            (bind _returnvalue (`self.K2_GetActorLocation` _output_3))
            (set `self.Min` (`KismetMathLibrary.VSize` (- (`self.K2_GetActorLocation` (`self.Pacman`)) _returnvalue)) :!label _label_2)
            (bind _output_get (set `local.Closet point` _output_3))
            (`KismetSystemLibrary.PrintString` (`KismetSystemLibrary.GetDisplayName` _output_get)))
          (:`CastFailed`
            (if (<= (`KismetMathLibrary.VSize` (- _location _returnvalue)) 0.0)
              (goto _label_2)))))
      (elif (> (`self.Min`) (`KismetMathLibrary.VSize` (- (`self.K2_GetActorLocation` (`self.Pacman`)) (`self.K2_GetActorLocation` _output_3))))
        (goto _label))))
  (set `local.Closet point` _closet_point)
  (return _closet_point))

(fn `Get Spherical Distance`
  (params (A :type "Vector Structure") (B :type "Vector Structure"))
  (returns (Distance :type "Float (double-precision)"))
  (return (* (`.SphereRadius` (`KismetSystemLibrary.GetComponentBounds` (`SphereMapBaseA.MeshComponent` (`self.Map`)))) (`KismetMathLibrary.Atan2` (`KismetMathLibrary.VSize` (`KismetMathLibrary.Cross_VectorVector` A B)) (`KismetMathLibrary.Dot_VectorVector` A B)))))

(fn `UserConstructionScript`)