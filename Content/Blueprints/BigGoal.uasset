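; BigGoal is a collectible power-up, similar to a power pellet, for a GearVR game with ghost-style enemies.
; On collection it adds 250 to the player character's score, makes every Enemy damageable with a blinking ghost material, then destroys itself.
; A timed branch meant to restore enemy invulnerability and material is unconnected, so this asset never reverts that state.
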(event `self.OnGetCollected`
  (bind _asgear_vrcharacter (cast `GearVRCharacter` (`GameplayStatics.GetPlayerCharacter` 0)))
  (`GearVRCharacter.UpdateScore` _asgear_vrcharacter 250)
  (bind _outactors (`GameplayStatics.GetAllActorsOfClass` "/Script/GearVRGame.Enemy"))
  (for _array_element _outactors
    (set `Enemy.bCanTakeDamage` true _array_element)
    (bind _mesh (`Character.Mesh` _array_element))
    (set `self.mat` (`PrimitiveComponent.GetMaterial` _mesh 0))
    (`PrimitiveComponent.SetMaterial` _mesh 0 "/Game/Blueprints/M_GhostBlink.M_GhostBlink"))
  (`self.K2_DestroyActor`))

(fn `UserConstructionScript`)