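; MenuActor is a VR pause menu shown on a stereo layer, with New Game and Exit buttons.
; BeginPlay places the layer at the player pawn's transform, lets it tick while paused and binds the MenuWidget buttons.
; Tick copies the widget's render target to the layer while paused and hides it otherwise.
; New Game unpauses and only prints "Open Level", Exit quits, and a Pac-Man lives-widget loop is left disconnected.
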(event `self.ReceiveBeginPlay`
  (bind _returnvalue (`self.GetTransform` (`GameplayStatics.GetPlayerPawn` 0)))
  ;[0.7474 1 0.4152] VR Menu Transform
  (`SceneComponent.K2_SetRelativeTransform` (`self.StereoLayer`) (`KismetMathLibrary.MakeTransform` (`KismetMathLibrary.MakeVector` (.x (.location _returnvalue)) (.y (.location _returnvalue)) (.z (.location _returnvalue))) (`KismetMathLibrary.MakeRotator` (.roll (.rotation _returnvalue)) (.pitch (.rotation _returnvalue)) (.yaw (.rotation _returnvalue)))) false false)
  (`ActorComponent.SetTickableWhenPaused` (`self.StereoLayer`) true)
  (`ActorComponent.SetTickableWhenPaused` (`self.Widget`) true)
  (`self.SetTickableWhenPaused` self true)
  (bind _asmenu_widget (cast `/Game/Blueprints/Menu/MenuWidget` (`WidgetComponent.GetUserWidgetObject` (`self.Widget`))))
  (add `Button.OnClicked` (`/Game/Blueprints/Menu/MenuWidget.NewGame` _asmenu_widget) (delegate `StartButtonClicked_Event`))
  (add `Button.OnClicked` (`/Game/Blueprints/Menu/MenuWidget.ExitGame` _asmenu_widget) (delegate `ExitButtonClicked_Event`)))

(event `StartButtonClicked_Event`
  (`GameplayStatics.SetGamePaused` false)
  (`ActorComponent.K2_DestroyComponent` (`self.Widget`))
  (`KismetSystemLibrary.PrintString` "Open Level"))

(event `self.ReceiveTick`
  (params (DeltaSeconds :type "Float (single-precision)"))
  (bind _widget (`self.Widget`))
  (if (`GameplayStatics.IsGamePaused`)
    (`/Engine/EditorBlueprintResources/StandardMacros.IsValid` _widget
      (:`Is Valid`
        (`StereoLayerComponent.SetTexture` (`self.StereoLayer`) (`WidgetComponent.GetRenderTarget` _widget))))
    (else
      (`SceneComponent.SetVisibility` (`self.StereoLayer`) false false))))

(event `ExitButtonClicked_Event`
  (`KismetSystemLibrary.QuitGame` null "Quit"))

(fn `UserConstructionScript`)