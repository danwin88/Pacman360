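; Game mode for a GearVR Pac-Man-style game that drives ghost spawning and handles level completion.
; BeginPlay starts a looping timer that calls GhostSpawn on the first GhostSpawner found.
; Tick polls for remaining GoalPickup actors; when none remain, it saves the player's score if it beats the stored best, then resets and restarts the game.
; The restart only runs if an existing save loads successfully.
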(event `self.ReceiveTick`
  (params (DeltaSeconds :type "Float (single-precision)"))
  (bind _outactors (`GameplayStatics.GetAllActorsOfClass` "/Script/GearVRGame.GoalPickup"))
  (if (<= (`KismetArrayLibrary.Array_Length` _outactors) 0)
    (bind _asbp_gear_vrgame_game_mode_base (cast `/Game/Blueprints/BP_GearVRGameGameModeBase` (`GameplayStatics.GetGameMode`)))
    (bind _asbp_pacman_character (cast `/Game/Blueprints/BP_Pacman_Character` (`GameplayStatics.GetPlayerCharacter` 0)))
    (bind _returnvalue (`GearVRCharacter.GetScore` _asbp_pacman_character))
    (bind _returnvalue_2 (`GameplayStatics.LoadGameFromSlot` "MySave"))
    (bind _asgear_vrsave_game (cast `/Game/Blueprints/GearVRSaveGame` _returnvalue_2))
    (if (> _returnvalue (`/Game/Blueprints/GearVRSaveGame.Best Score` _asgear_vrsave_game))
      (bind _returnvalue_3 (`GameplayStatics.CreateSaveGameObject` "/Game/Blueprints/GearVRSaveGame.GearVRSaveGame_C"))
      (set `/Game/Blueprints/GearVRSaveGame.Best Score` _returnvalue _returnvalue_3)
      (`GameplayStatics.SaveGameToSlot` _returnvalue_3 "MySave"))
    (`self.ResetLevel` _asbp_gear_vrgame_game_mode_base)
    (`self.RestartGame` _asbp_gear_vrgame_game_mode_base)))

(event `self.ReceiveBeginPlay`
  (bind _outactors (`GameplayStatics.GetAllActorsOfClass` "/Game/Blueprints/GhostSpawner.GhostSpawner_C"))
  (`KismetSystemLibrary.K2_SetTimer` (`|GetArrayItem` _outactors) "GhostSpawn" 5.0 true))

(fn `UserConstructionScript`)